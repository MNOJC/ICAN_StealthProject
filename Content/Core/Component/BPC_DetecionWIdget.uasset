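; Widget component that briefly displays a detection marker on its owning actor, sized to that actor's mesh.
; BeginPlay derives a base draw size from the owner's mesh bounds, using the larger horizontal extent for width and vertical extent for height.
; DetectedEffect shows the widget and enables tick for one second, then hides it and disables tick.
; While ticking, draw size shrinks as the player pawn's distance to the owner grows, within clamped limits.
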(event `self.ReceiveBeginPlay`
  (set `self.Size` (`KismetMathLibrary.MakeVector2D` (* (`KismetMathLibrary.FMax` (.x (* (`.BoxExtent` (`KismetSystemLibrary.GetComponentBounds` (`Actor.GetComponentByClass` (`self.GetOwner`) "/Script/Engine.MeshComponent"))) 5.0)) (.y (* (`.BoxExtent` (`KismetSystemLibrary.GetComponentBounds` (`Actor.GetComponentByClass` (`self.GetOwner`) "/Script/Engine.MeshComponent"))) 5.0))) 3.0) (.z (* (`.BoxExtent` (`KismetSystemLibrary.GetComponentBounds` (`Actor.GetComponentByClass` (`self.GetOwner`) "/Script/Engine.MeshComponent"))) 5.0)))))

(event `Detected Effect`
  (`self.SetComponentTickEnabled` true)
  (`self.SetVisibility` true)
  (`KismetSystemLibrary.Delay` 1.0)
  (`self.SetVisibility` false)
  (`self.SetComponentTickEnabled` false))

(event `self.ReceiveTick`
  (params (DeltaSeconds :type "Float (single-precision)"))
  (`self.SetDrawSize` (* (`self.Size`) (`KismetMathLibrary.Lerp` 2.0 0.2 (`KismetMathLibrary.FClamp` (/ (`Actor.GetDistanceTo` (`GameplayStatics.GetPlayerPawn` 0) (`self.GetOwner`)) 1000.0))))))