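; BP_Player is the player character Blueprint, handling camera adjustments and spawning a controllable robot.
; Timelines animate a shoulder swap on the camera boom and a crouch offset on the follow camera, though the node caching the camera's default location is disconnected.
; Spawning creates one BP_Robot at a time and possesses it, clearing the guard flag when it is destroyed.
; Mouse-look and BeginPlay are empty, and Scan returns only constant values.
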(event `EnhancedInput|/Game/Input/Actions/IA_SwapCameraOffset`
  (params (ActionValue :type Boolean) (ElapsedSeconds :type "Float (double-precision)") (TriggeredSeconds :type "Float (double-precision)") (InputAction :type "InputAction Object Reference" :default "/Game/Input/Actions/IA_SwapCameraOffset.IA_SwapCameraOffset"))
  (:`Started`
    (bind _output_get (set `self.FlipFlop` (not (`self.FlipFlop`))))
    (if _output_get
      (bind (_direction _value) (`Timeline|SwapCamera` :!label _label)
        (:`Update`
          (set `SpringArmComponent.SocketOffset` (`KismetMathLibrary.MakeVector` 0.0 (`KismetMathLibrary.Lerp` 40.0 -40.0 _value) 90.0) (`self.CameraBoom`))))
      (else
        (goto _label :!via `Reverse`)))))

(event `EnhancedInput|/Game/Input/Actions/IA_MouseLook`
  (params (ActionValue :type "Vector2D Structure") (ElapsedSeconds :type "Float (double-precision)") (TriggeredSeconds :type "Float (double-precision)") (InputAction :type "InputAction Object Reference" :default "/Game/Input/Actions/IA_MouseLook.IA_MouseLook")))

(event `self.ReceiveBeginPlay`)

(event `EnhancedInput|/Game/Input/Actions/IA_Crouch` :!enabledstate Disabled
  (params (ActionValue :type Boolean) (ElapsedSeconds :type "Float (double-precision)") (TriggeredSeconds :type "Float (double-precision)") (InputAction :type "InputAction Object Reference" :default "/Game/Input/Actions/IA_Crouch.IA_Crouch"))
  (bind _defaultcamerarelativelocation (`self.DefaultCameraRelativeLocation`))
  (:`Triggered`
    (if (not (`NavMovementComponent.IsCrouching` (`self.CharacterMovement`)))
      (bind (_direction _alpha) (`Timeline|CameraTransition` :!label _label_2)
        (:`Update`
          (`SceneComponent.K2_SetRelativeLocation` (`self.FollowCamera`) (`KismetMathLibrary.VLerp` _defaultcamerarelativelocation (+ _defaultcamerarelativelocation (`self.Crouched CameraRelativeLocationOffset`)) _alpha) false false)))
      (else
        (goto _label_2 :!via `Reverse`)))))

(event `EnhancedInput|/Game/Input/Actions/IA_SpawnRobot`
  (params (ActionValue :type Boolean) (ElapsedSeconds :type "Float (double-precision)") (TriggeredSeconds :type "Float (double-precision)") (InputAction :type "InputAction Object Reference" :default "/Game/Input/Actions/IA_SpawnRobot.IA_SpawnRobot"))
  (:`Triggered`
    (if (not (`self.RobotSpawned`))
      (set `self.RobotSpawned` true)
      (bind _returnvalue (`|SpawnActorFromClass` "/Game/Core/Classes/Characters/BP_Robot.BP_Robot_C" (`self.GetTransform`) "AdjustIfPossibleButAlwaysSpawn" "MultiplyWithRoot" null self null))
      (`Controller.Possess` (`self.GetController`) _returnvalue)
      (add `self.OnDestroyed` _returnvalue (delegate `OnDestroy`)))))

(event `OnDestroy` :!signature `self.OnDestroyed`
  (params (DestroyedActor :type "Actor Object Reference"))
  (set `self.RobotSpawned` false))

(fn `Scan`
  (returns (Type :type "/Game/Core/Enum/E_EntityType Enum") (HitLocation :type "Vector Structure"))
  (return "NewEnumerator0" (0.0 0.0 0.0)))

(fn `UserConstructionScript`
  (`parent.UserConstructionScript`))