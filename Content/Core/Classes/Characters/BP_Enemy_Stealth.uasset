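; Stealth enemy character that patrols under AI control and can be scanned or temporarily knocked down.
; BeginPlay seeds the blackboard with patrol type and spawn transform, then caches its AI_Enemy controller.
; TriggerObject switches the controller's activate state, hides the spotlight and plays a death montage, reverting all three after a delay.
; Scan fires the detection widget effect, reveals a plane and returns a type and the actor's location.
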(event `self.ReceiveBeginPlay`
  (bind _returnvalue (`AIBlueprintHelperLibrary.GetBlackboard` (`AIBlueprintHelperLibrary.GetAIController` self)))
  (`BlackboardComponent.SetValueAsEnum` (`AIBlueprintHelperLibrary.GetBlackboard` (`AIBlueprintHelperLibrary.GetAIController` self)) "PatrolType" (`self.PatrolType`))
  (`BlackboardComponent.SetValueAsVector` _returnvalue "StaticPatrolLocation" (`self.K2_GetActorLocation`))
  (`BlackboardComponent.SetValueAsRotator` _returnvalue "StaticPatrolRotation" (`self.K2_GetActorRotation`))
  (bind _asai_enemy (cast `/Game/AI/Controller/AI_Enemy` (`AIBlueprintHelperLibrary.GetAIController` self)))
  (set `self.As AI Enemy` _asai_enemy))

(event `/Game/AI/Behavior/Gameplay/Interface/BPI_Interactible.TriggerObject`
  (`/Game/AI/Controller/AI_Enemy.SetActivateState` (`self.As AI Enemy`) true)
  (`SceneComponent.SetVisibility` (`self.SpotLight`) false false)
  (`|PlayMontage` (`self.Mesh`) "/Game/Fab/MCO_Mocap_Basics/Animation/Mobility_Pro/Root_Motion/MOB1_Stand_Relaxed_Death_B_Montage.MOB1_Stand_Relaxed_Death_B_Montage"
    (:`then`
      (`KismetSystemLibrary.Delay` 15.0)
      (`self.StopAnimMontage` "/Game/Fab/MCO_Mocap_Basics/Animation/Mobility_Pro/Root_Motion/MOB1_Stand_Relaxed_Death_B_Montage.MOB1_Stand_Relaxed_Death_B_Montage")
      (`/Game/AI/Controller/AI_Enemy.SetActivateState` (`self.As AI Enemy`) false)
      (`SceneComponent.SetVisibility` (`self.SpotLight`) true false))))

(fn `Scan`
  (returns (Type :type "/Game/Core/Enum/E_EntityType Enum") (HitLocation :type "Vector Structure"))
  (`/Game/Core/Component/BPC_DetecionWIdget.Detected Effect` (`self.BPC_DetecionWIdget`))
  (`SceneComponent.SetVisibility` (`self.Plane`) true false)
  (return "NewEnumerator2" (`self.K2_GetActorLocation`)))

(fn `UserConstructionScript`)