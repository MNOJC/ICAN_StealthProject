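; Possessable robot character, with its own input context and HUD, that publishes its position to the scan material parameter collection every tick.
; Holding zoom narrows FOV to arm interaction, which sphere-traces from the camera to trigger hit objects; a detection count also toggles that permission.
; A timeline swaps the camera shoulder offset.
; Spawn input returns control to the player; on unpossession, a spawned AI controller walks the robot to them and destroys it.
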(event `self.ReceiveTick`
  (params (DeltaSeconds :type "Float (single-precision)"))
  (bind (_returnvalue_x _returnvalue_y _returnvalue_z) (`KismetMathLibrary.BreakVector` (`self.K2_GetActorLocation`)))
  (`KismetSystemLibrary.PrintString` (`KismetStringLibrary.Conv_IntToString` (`self.DetectedCount`)) true true (struct :`R` 1.0 :`G` 0.044426 :`A` 1.0) 0.0)
  (`KismetMaterialLibrary.SetVectorParameterValue` "/Game/Art/Material/MPC_Scan.MPC_Scan" "Position" (make `LinearColor` _returnvalue_x _returnvalue_y _returnvalue_z 1.0)))

(event `self.ReceiveUnpossessed`
  (params (OldController :type "Controller Object Reference"))
  (bind _foundwidgets (`WidgetBlueprintLibrary.GetAllWidgetsOfClass` "/Game/Core/UI/Molecule/WBP_Doghud.WBP_Doghud_C"))
  (bind _output (`|GetArrayItem` _foundwidgets))
  (`/Engine/EditorBlueprintResources/StandardMacros.IsValid` _output
    (:`Is Valid`
      (`Widget.RemoveFromParent` _output)
      (`KismetSystemLibrary.CollectGarbage`)
      (message `EnhancedInputSubsystemInterface.RemoveMappingContext` (pcsubsystem `EnhancedInputLocalPlayerSubsystem` (`GameplayStatics.GetPlayerController` 0)) "/Game/Input/IMC_Robot.IMC_Robot" (struct))
      (bind _returnvalue (`|SpawnActorFromClass` "/Script/AIModule.AIController" (`KismetMathLibrary.MakeTransform` (0.0 0.0 0.0)) "AlwaysSpawn" "MultiplyWithRoot" null null))
      (`KismetSystemLibrary.DelayUntilNextTick`)
      (`Controller.Possess` _returnvalue self)
      (`|AIMoveTo` self (0.0 0.0 0.0) (`self.Player`) 10.0
        (:`OnSuccess`
          (`self.K2_DestroyActor`))))))

(event `self.ReceivePossessed`
  (params (NewController :type "Controller Object Reference"))
  (if (== NewController (`GameplayStatics.GetPlayerController` 0))
    (message `EnhancedInputSubsystemInterface.AddMappingContext` (pcsubsystem `EnhancedInputLocalPlayerSubsystem` (`GameplayStatics.GetPlayerController` 0)) "/Game/Input/IMC_Robot.IMC_Robot" 0 (struct))
    (bind _returnvalue (`|CreateWidget` "/Game/Core/UI/Molecule/WBP_Doghud.WBP_Doghud_C"))
    (`UserWidget.AddToViewport` _returnvalue 0)))

(event `EnhancedInput|/Game/Input/Actions/IA_SpawnRobot`
  (params (ActionValue :type Boolean) (ElapsedSeconds :type "Float (double-precision)") (TriggeredSeconds :type "Float (double-precision)") (InputAction :type "InputAction Object Reference" :default "/Game/Input/Actions/IA_SpawnRobot.IA_SpawnRobot"))
  (:`Triggered`
    (`Controller.Possess` (`self.GetController`) (`self.Player`))))

(event `EnhancedInput|/Game/Input/Actions/IA_InteractZoom`
  (params (ActionValue :type Boolean) (ElapsedSeconds :type "Float (double-precision)") (TriggeredSeconds :type "Float (double-precision)") (InputAction :type "InputAction Object Reference" :default "/Game/Input/Actions/IA_InteractZoom.IA_InteractZoom"))
  (:`Started`
    (`TimelineComponent.SetPlayRate` (`self.Interaction Zoom`) (/ 1.0 (`self.Interaction Delay`)))
    (bind (_direction _value_0_1) (`Timeline|Interaction Zoom` :!label _label)
      (:`Update`
        (`CameraComponent.SetFieldOfView` (`self.Camera`) (`KismetMathLibrary.Lerp` 90.0 60.0 _value_0_1)))
      (:`Finished`
        (if ActionValue
          (set `self.Can Interact` true)))))
  (:`Completed`
    (set `self.Can Interact` false)
    (goto _label :!via `Reverse`)))

(event `EnhancedInput|/Game/Input/Actions/IA_SwapCameraOffset`
  (params (ActionValue :type Boolean) (ElapsedSeconds :type "Float (double-precision)") (TriggeredSeconds :type "Float (double-precision)") (InputAction :type "InputAction Object Reference" :default "/Game/Input/Actions/IA_SwapCameraOffset.IA_SwapCameraOffset"))
  (:`Started`
    (bind _output_get (set `self.FlipFlop` (not (`self.FlipFlop`))))
    (if _output_get
      (bind (_direction _value) (`Timeline|Timeline_0` :!label _label_2)
        (:`Update`
          (set `SpringArmComponent.SocketOffset` (`KismetMathLibrary.MakeVector` 180.0 (`KismetMathLibrary.Lerp` 20.0 -20.0 _value) 30.0) (`self.CameraBoom`))))
      (else
        (goto _label_2 :!via `Reverse`)))))

(event `EnhancedInput|/Game/Input/Actions/IA_Interact`
  (params (ActionValue :type Boolean) (ElapsedSeconds :type "Float (double-precision)") (TriggeredSeconds :type "Float (double-precision)") (InputAction :type "InputAction Object Reference" :default "/Game/Input/Actions/IA_Interact.IA_Interact"))
  (bind _transformcomponent (`PlayerCameraManager.TransformComponent` (`GameplayStatics.GetPlayerCameraManager` 0)))
  (bind _returnvalue (`SceneComponent.K2_GetComponentLocation` _transformcomponent))
  (:`Triggered`
    (if (`self.Can Interact`)
      (bind _outhits (`KismetSystemLibrary.SphereTraceMulti` :`Start` _returnvalue :`End` (+ _returnvalue (* (`SceneComponent.GetForwardVector` _transformcomponent) (`self.Range`))) :`Radius` 30.0 :`TraceChannel` "TraceTypeQuery3" :`DrawDebugType` "ForDuration" :`DrawTime` 1.0))
      (for _array_element _outhits
        (message `/Game/AI/Behavior/Gameplay/Interface/BPI_Interactible.TriggerObject` (`.HitActor` (`GameplayStatics.BreakHitResult` _array_element)))))))

(event `EnhancedInput|/Game/Input/Actions/IA_MouseLook`
  (params (ActionValue :type "Vector2D Structure") (ElapsedSeconds :type "Float (double-precision)") (TriggeredSeconds :type "Float (double-precision)") (InputAction :type "InputAction Object Reference" :default "/Game/Input/Actions/IA_MouseLook.IA_MouseLook")))

(fn `UpdateDetectedCount`
  (params (Add :type Boolean))
  (bind _detectedcount (`self.DetectedCount`))
  (if Add
    (bind _result (`/Engine/EditorBlueprintResources/StandardMacros.IncrementInt` _detectedcount)
      (:`  `
        (set `self.DetectedCount` (`KismetMathLibrary.Clamp` _result 0 99))))
    (else
      (bind _result_2 (`/Engine/EditorBlueprintResources/StandardMacros.DecrementInt` _detectedcount)
        (:`  `
          (set `self.DetectedCount` (`KismetMathLibrary.Clamp` _result_2 0 99))))))
  (if (== (`self.DetectedCount`) 0)
    (set `self.Can Interact` true)
    (else
      (set `self.Can Interact` false))))

(fn `UserConstructionScript`)