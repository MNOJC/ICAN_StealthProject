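; BP_End is a level exit that starts a win countdown when an actor of the configured class overlaps it.
; The WinDelay timeline drives a WBP_Timer widget showing the rounded-up time.
; On finish it pauses the game while async loading NextLevel, then unpauses and opens that level.
; Leaving the overlap removes the widget, forces garbage collection and stops the timeline, which restarts from zero on re-entry.
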(event `self.ReceiveActorBeginOverlap`
  (params (OtherActor :type "Actor Object Reference"))
  (if (== (`GameplayStatics.GetObjectClass` OtherActor) (`|ConvertAsset` (`self.Class`)))
    (bind _returnvalue (`|CreateWidget` "/Game/Core/UI/HUD/WBP_Timer.WBP_Timer_C"))
    (`UserWidget.AddToViewport` _returnvalue 3)
    (set `self.Timer` _returnvalue)
    (bind (_direction _time) (`Timeline|Win Delay` :!via `PlayFromStart` :!label _label)
      (:`Update`
        (`TextBlock.SetText` (`/Game/Core/UI/HUD/WBP_Timer.TextBlock_54` (`self.Timer`)) (`KismetTextLibrary.Conv_IntToText` (`KismetMathLibrary.FCeil` _time))))
      (:`Finished`
        (`|LoadAsset` (`self.NextLevel`)
          (:`then`
            (`GameplayStatics.SetGamePaused` true))
          (:`Completed`
            (`GameplayStatics.SetGamePaused` false)
            (`GameplayStatics.OpenLevelBySoftObjectPtr` (`self.NextLevel`))))))))

(event `self.ReceiveActorEndOverlap`
  (params (OtherActor :type "Actor Object Reference"))
  (if (== (`GameplayStatics.GetObjectClass` OtherActor) (`|ConvertAsset` (`self.Class`)))
    (`Widget.RemoveFromParent` (`self.Timer`))
    (`KismetSystemLibrary.CollectGarbage`)
    (goto _label :!via `Stop`)))

(fn `UserConstructionScript`)