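; BP_SAS_START is a start airlock door actor that opens on its own shortly after play begins.
; After a short delay on BeginPlay, it stores the door mesh's starting height and plays a timeline at half speed.
; Each timeline update offsets the door's world Z from that height by the track value, sliding it vertically.
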(event `self.ReceiveBeginPlay`
  (bind _sm_door_2_merged_staticmeshcomponent0 (`self.SM_Door_2_Merged_StaticMeshComponent0`))
  (bind (_returnvalue_x _returnvalue_y _returnvalue_z) (`KismetMathLibrary.BreakVector` (`SceneComponent.K2_GetComponentLocation` _sm_door_2_merged_staticmeshcomponent0)))
  (`KismetSystemLibrary.Delay` 3.0)
  (set `self.InitialZ` _returnvalue_z)
  (`TimelineComponent.SetPlayRate` (`self.Timeline`) 0.5)
  (bind (_direction _newtrack_0) (`Timeline|Timeline`)
    (:`Update`
      (`SceneComponent.K2_SetWorldLocation` _sm_door_2_merged_staticmeshcomponent0 (`KismetMathLibrary.MakeVector` _returnvalue_x _returnvalue_y (+ (`self.InitialZ`) (* _newtrack_0 250.0))) false false))))

(fn `UserConstructionScript`
  (`parent.UserConstructionScript`))