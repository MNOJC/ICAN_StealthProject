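; EQS context that gives an enemy a predicted location for the player from its AI controller's last seen position, direction and velocity.
; A visibility trace projects ahead by 1.5 times the last speed, stopping at obstacles.
; A second trace seeks the ground, but scales its offset from the point's world coordinates, so it is not strictly vertical.
; It returns that point raised 120 units, with debug drawing of traces and result.
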(fn `ProvideSingleLocation`
  (params (QuerierObject :type "Object Object Reference") (QuerierActor :type "Actor Object Reference"))
  (returns (ResultingLocation :type "Vector Structure"))
  (locals (FirstPoint :type "Vector Structure" :default (0.0 0.0 0.0)) (SecondPoint :type "Vector Structure"))
  (bind _firstpoint (`local.FirstPoint`))
  (bind _returnvalue (`KismetMathLibrary.MakeVector` (.x (`local.SecondPoint`)) (.y (`local.SecondPoint`)) (+ (.z (`local.SecondPoint`)) 120.0)))
  (bind _asbp_enemy (cast `/Game/AI/Enemy/BP_Enemy` QuerierObject))
  (bind _asai_enemy (cast `/Game/AI/Controller/AI_Enemy` (`AIBlueprintHelperLibrary.GetAIController` _asbp_enemy)))
  (bind _lastplayerlocation (`/Game/AI/Controller/AI_Enemy.LastPlayerLocation` _asai_enemy))
  (bind (_outhit _returnvalue_2) (`KismetSystemLibrary.LineTraceSingle` :`Start` _lastplayerlocation :`End` (+ (* (`/Game/AI/Controller/AI_Enemy.LastPlayerDirection` _asai_enemy) (* (`KismetMathLibrary.VSize` (`/Game/AI/Controller/AI_Enemy.LastPlayerVelocity` _asai_enemy)) 1.5)) _lastplayerlocation) :`TraceChannel` "TraceTypeQuery1" :`DrawDebugType` "ForDuration"))
  (if _returnvalue_2
    (bind (_bblockinghit _binitialoverlap _time _distance _location _impactpoint _normal _impactnormal _physmat _hitactor _hitcomponent _hitbonename _bonename _hititem _elementindex _faceindex _tracestart _traceend) (`GameplayStatics.BreakHitResult` _outhit))
    (set `local.FirstPoint` _location)
    (else
      (set `local.FirstPoint` _traceend)))
  (bind (_outhit_2 _returnvalue_3) (`KismetSystemLibrary.LineTraceSingle` :`Start` _firstpoint :`End` (+ _firstpoint (* _firstpoint (1.0 1.0 -1000.0))) :`TraceChannel` "TraceTypeQuery1" :`DrawDebugType` "ForDuration"))
  (if _returnvalue_3
    (bind (_bblockinghit_2 _binitialoverlap_2 _time_2 _distance_2 _location_2 _impactpoint_2 _normal_2 _impactnormal_2 _physmat_2 _hitactor_2 _hitcomponent_2 _hitbonename_2 _bonename_2 _hititem_2 _elementindex_2 _faceindex_2 _tracestart_2 _traceend_2) (`GameplayStatics.BreakHitResult` _outhit_2))
    (set `local.SecondPoint` _location_2)
    (else
      (set `local.SecondPoint` _traceend_2)))
  (`KismetSystemLibrary.DrawDebugSphere` _returnvalue 20.0 12 (struct :`R` 0.56238 :`B` 1.0 :`A` 1.0) 5.0 5.0)
  (return _returnvalue))