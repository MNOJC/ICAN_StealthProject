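; Security camera smart object that sweeps between two rotations and detects the player through an overlap cone.
; A state enum drives Tick rotation and cone color: look around, timed analysis, yaw-clamped player tracking, or broken.
; Tracking starts a looping MakeNoise beep instigated by the player, and leaving the cone starts a delayed return to sweeping.
; TriggerObject breaks the camera and makes stealth enemies' AI perception forget everything.
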(event `self.ReceiveBeginPlay`
  (bind _yaw (.yaw (`self.StartWorldRotation`)))
  (set `self.TargetCameraRotation` (`self.CameraRotationMax`))
  (`self.UpdateCameraState` "NewEnumerator0")
  (set `self.StartWorldRotation` (`SceneComponent.K2_GetComponentRotation` (`self.Camera`)))
  (`AIPerceptionStimuliSourceComponent.RegisterForSense` (`self.AIPerceptionStimuliSource`) "/Script/AIModule.AISense_Sight")
  (set `self.MIN` (+ _yaw -70.0))
  (set `self.MAX` (+ _yaw 70.0)))

(event `self.ReceiveTick`
  (params (DeltaSeconds :type "Float (single-precision)"))
  (bind _camerastate (`self.CameraState`))
  (bind _camera (`self.Camera`))
  (bind _returnvalue (`KismetMathLibrary.RInterpTo_Constant` (`SceneComponent.RelativeRotation` (`self.Camera`)) (`self.TargetCameraRotation`) (`GameplayStatics.GetWorldDeltaSeconds`) (`self.RotationSpeed`)))
  (set `self.currentworld rotation` (`SceneComponent.K2_GetComponentRotation` (`self.Camera`)))
  (if (or (`|EnumEquality` _camerastate "NewEnumerator0") (`|EnumEquality` _camerastate "NewEnumerator3"))
    (`SceneComponent.K2_SetRelativeRotation` (`self.Camera`) _returnvalue false false)
    (`SceneComponent.K2_SetRelativeRotation` (`self.Camera`) _returnvalue false false)
    (if (== _returnvalue (`self.CameraRotationMax`) :`ErrorTolerance` 1.0)
      (set `self.TargetCameraRotation` (`self.CameraRotationMin`))
      (elif (== _returnvalue (`self.CameraRotationMin`) :`ErrorTolerance` 1.0)
        (set `self.TargetCameraRotation` (`self.CameraRotationMax`))))
    (elif (`|EnumEquality` _camerastate "NewEnumerator1")
      (`SceneComponent.K2_SetWorldRotation` (`self.Camera`) (`KismetMathLibrary.MakeRotator` (.roll (`KismetMathLibrary.RLerp` (`SceneComponent.K2_GetComponentRotation` _camera) (`KismetMathLibrary.MakeRotator` 0.0 0.0 (+ (.yaw (`KismetMathLibrary.FindLookAtRotation` (`SceneComponent.K2_GetComponentLocation` _camera) (`self.K2_GetActorLocation` (`self.As BP Player`)))) -90.0)) (* (`GameplayStatics.GetWorldDeltaSeconds`) 5.0) true)) (.pitch (`KismetMathLibrary.RLerp` (`SceneComponent.K2_GetComponentRotation` _camera) (`KismetMathLibrary.MakeRotator` 0.0 0.0 (+ (.yaw (`KismetMathLibrary.FindLookAtRotation` (`SceneComponent.K2_GetComponentLocation` _camera) (`self.K2_GetActorLocation` (`self.As BP Player`)))) -90.0)) (* (`GameplayStatics.GetWorldDeltaSeconds`) 5.0) true)) (`KismetMathLibrary.FClamp` (.yaw (`KismetMathLibrary.RLerp` (`SceneComponent.K2_GetComponentRotation` _camera) (`KismetMathLibrary.MakeRotator` 0.0 0.0 (+ (.yaw (`KismetMathLibrary.FindLookAtRotation` (`SceneComponent.K2_GetComponentLocation` _camera) (`self.K2_GetActorLocation` (`self.As BP Player`)))) -90.0)) (* (`GameplayStatics.GetWorldDeltaSeconds`) 5.0) true)) (`self.MIN`) (`self.MAX`))) false false))))

(event `self.ConeDetection.OnComponentBeginOverlap`
  (params (OverlappedComponent :type "PrimitiveComponent Object Reference") (OtherActor :type "Actor Object Reference") (OtherComp :type "PrimitiveComponent Object Reference") (OtherBodyIndex :type Integer) (bFromSweep :type Boolean) (SweepResult :type "HitResult Structure (by ref)"))
  (bind _camerastate (`self.CameraState`))
  (bind _asbp_player (cast `/Game/Core/Classes/Characters/BP_Player` OtherActor))
  (set `self.As BP Player` _asbp_player)
  (if (and (`|EnumInequality` _camerastate "NewEnumerator1") (`|EnumInequality` _camerastate "NewEnumerator2"))
    (`self.UpdateCameraState` "NewEnumerator3")
    (`self.StartAnalyse`)))

(event `StartAnalyse`
  (bind _returnvalue (`KismetSystemLibrary.K2_SetTimerDelegate` (delegate `TriggerCamera`) 1.0))
  (set `self.TimerHandle` _returnvalue))

(event `self.ConeDetection.OnComponentEndOverlap`
  (params (OverlappedComponent :type "PrimitiveComponent Object Reference") (OtherActor :type "Actor Object Reference") (OtherComp :type "PrimitiveComponent Object Reference") (OtherBodyIndex :type Integer))
  (bind _camerastate (`self.CameraState`))
  (cast `/Game/Core/Classes/Characters/BP_Player` OtherActor)
  (if (and (`|EnumInequality` _camerastate "NewEnumerator1") (`|EnumInequality` _camerastate "NewEnumerator2"))
    (`self.UpdateCameraState` "NewEnumerator0")
    (`KismetSystemLibrary.K2_ClearAndInvalidateTimerHandle` (`self.TimerHandle`))
    (elif (`|EnumInequality` _camerastate "NewEnumerator2")
      (`self.StartLoseSight`))))

(event `StartLoseSight`
  (bind _returnvalue (`KismetSystemLibrary.K2_SetTimerDelegate` (delegate `LoseSight`) 3.0))
  (set `self.LoseSightHandle` _returnvalue))

(event `TriggerCamera`
  (`self.UpdateCameraState` "NewEnumerator1")
  (`self.StartBIP`))

(event `LoseSight`
  (`self.UpdateCameraState` "NewEnumerator0"))

(event `StartBIP`
  (bind _returnvalue (`KismetSystemLibrary.K2_SetTimerDelegate` (delegate `BIPInterval`) 0.4 true))
  (set `self.BIPTimerHandle` _returnvalue))

(event `/Game/AI/Behavior/Gameplay/Interface/BPI_Interactible.TriggerObject`
  (`self.BreakCamera`))

(event `BIPInterval`
  (`self.MakeNoise` 10.0 (`GameplayStatics.GetPlayerCharacter` 0) (`self.K2_GetActorLocation`)))

(event `self.SmartObject.OnSmartObjectEvent`
  (params (EventData :type "SmartObjectEventData Structure (by ref)") (Interactor :type "Actor Object Reference")))

(fn `BreakCamera`
  (`self.UpdateCameraState` "NewEnumerator2")
  (bind _outactors (`GameplayStatics.GetAllActorsOfClass` "/Game/Core/Classes/Characters/BP_Enemy_Stealth.BP_Enemy_Stealth_C"))
  (for _array_element _outactors
    (bind _asai_enemy (cast `/Game/AI/Controller/AI_Enemy` (`AIBlueprintHelperLibrary.GetAIController` _array_element)))
    (`AIPerceptionComponent.ForgetAll` (`/Game/AI/Controller/AI_Enemy.AIPerception` _asai_enemy))))

(fn `Scan`
  (returns (Type :type "/Game/Core/Enum/E_EntityType Enum") (HitLocation :type "Vector Structure"))
  (return "NewEnumerator0" (0.0 0.0 0.0)))

(fn `UpdateCameraState`
  (params (CameraState :type "/Game/AI/Behavior/Gameplay/SmartObjects/Enums/ECameraState Enum" :default "NewEnumerator0"))
  (bind _camera (`self.Camera`))
  (bind (_relativerotation_roll _relativerotation_pitch _relativerotation_yaw) (`KismetMathLibrary.BreakRotator` (`SceneComponent.RelativeRotation` _camera)))
  (bind _output_get (set `self.CameraState` CameraState))
  (bind _returnvalue (`PrimitiveComponent.CreateDynamicMaterialInstance` (`self.ConeDetection`) 0 null "None"))
  (`MaterialInstanceDynamic.SetVectorParameterValue` _returnvalue "Color" (select `/Game/AI/Behavior/Gameplay/SmartObjects/Enums/ECameraState` _output_get :`NewEnumerator0` (struct :`R` 1.0 :`G` 1.0 :`B` 1.0 :`A` 1.0) :`NewEnumerator1` (struct :`R` 1.0 :`B` 0.008932 :`A` 1.0) :`NewEnumerator3` (struct :`R` 1.0 :`G` 0.619957 :`A` 1.0) :!type "LinearColor Structure"))
  (`SceneComponent.K2_SetRelativeRotation` _camera (`KismetMathLibrary.MakeRotator` (select `/Game/AI/Behavior/Gameplay/SmartObjects/Enums/ECameraState` _output_get :`NewEnumerator0` _relativerotation_roll :`NewEnumerator1` _relativerotation_roll :`NewEnumerator2` 70.0 :`NewEnumerator3` _relativerotation_roll) _relativerotation_pitch _relativerotation_yaw) false false)
  (`SceneComponent.SetVisibility` (`self.ConeDetection`) (select `/Game/AI/Behavior/Gameplay/SmartObjects/Enums/ECameraState` (`self.CameraState`) :`NewEnumerator0` true :`NewEnumerator1` true :`NewEnumerator2` true :`NewEnumerator3` true) false))

(fn `UserConstructionScript`)