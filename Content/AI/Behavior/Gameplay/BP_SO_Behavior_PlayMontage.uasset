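; Smart object behavior that has an AI avatar play a crouch idle montage to repair a BP_SO_Camera.
; When triggered, it casts the owner to the camera and plays the montage on the avatar's skeletal mesh.
; The CameraRepaired montage notify updates the camera's state and clears its CurrentlyRepair flag.
; The behavior ends when the montage completes or is interrupted.
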(event `self.K2_OnTriggeredCharacter`
  (params (Avatar :type "Character Object Reference") (Config :type "GameplayBehaviorConfig Object Reference") (SmartObjectOwner :type "Actor Object Reference"))
  (bind _asbp_so_camera (cast `/Game/AI/Behavior/Gameplay/SmartObjects/BP_SO_Camera` SmartObjectOwner))
  (set `self.Avatar` Avatar)
  (bind _notifyname (`|PlayMontage` (`Actor.GetComponentByClass` (`self.Avatar`) "/Script/Engine.SkeletalMeshComponent") "/Game/Fab/MCO_Mocap_Basics/Animation/Mobility_Pro/Root_Motion/MOB1_Crouch_Idle_V2_Montage.MOB1_Crouch_Idle_V2_Montage")
    (:`OnCompleted`
      (`self.K2_EndBehavior` (`self.Avatar`) :!label _label))
    (:`OnInterrupted`
      (goto _label))
    (:`OnNotifyBegin`
      (if (== _notifyname "CameraRepaired")
        (`/Game/AI/Behavior/Gameplay/SmartObjects/BP_SO_Camera.UpdateCameraState` _asbp_so_camera "NewEnumerator0")
        (set `/Game/AI/Behavior/Gameplay/SmartObjects/BP_SO_Camera.CurrentlyRepair` false _asbp_so_camera)))))