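; BP_SplinePatrol is an AI patrol route Blueprint built on a spline component.
; Its construction script rebuilds an array of the spline's points in world space and stores the last point index.
; The StartMethod enum then sets the spline shape: open for the back-and-forth modes, closed for the loop modes, whether starting from beginning or end.
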(fn `UserConstructionScript`
  (bind _spline (`self.Spline`))
  (`KismetArrayLibrary.Array_Clear` (`self.SplinePoints`))
  (bind _output_get (set `self.MaxSplinePointIndex` (- (`SplineComponent.GetNumberOfSplinePoints` (`self.Spline`)) 1)))
  (for _index (range (+ _output_get 1))
    (`KismetArrayLibrary.Array_Add` (`self.SplinePoints`) (`SplineComponent.GetSplinePointAt` (`self.Spline`) _index "World")))
  (switch `/Game/AI/Behavior/SplinePatrol/ESplinePatrolBehaviorMethod` (`self.StartMethod`)
    (:`NewEnumerator0`
      (`SplineComponent.SetClosedLoop` _spline false true :!label _label))
    (:`NewEnumerator1`
      (goto _label))
    (:`NewEnumerator2`
      (`SplineComponent.SetClosedLoop` _spline true true :!label _label_2))
    (:`NewEnumerator3`
      (goto _label_2))))